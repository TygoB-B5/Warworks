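; BP_TestBp is a test Blueprint for an AI-controlled character that moves to requested positions.
; OnRequestMoveTowards stores the 2D destination and issues a straight-line AI MoveToLocation without pathfinding.
; Tick checks whether the actor's 2D location nearly matches that destination, then halts movement and interpolates rotation toward the unset, default target rotation.
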(event EventTick
  (params (DeltaSeconds :type Float%20%28single-precision%29))
  (if (Utilities|Operators|EqualEqual (Variables|Default|GetDestination) (Math|Conversions|ToVector2D(Vector) (Transformation|GetActorLocation)) 0.1)
    (Transformation|SetActorRotation (Math|Interpolation|RInterpTo (Transformation|GetActorRotation) "0, 0, 0" DeltaSeconds 5.0) true)
    (Components|Movement|StopMovementImmediately (Variables|Character|GetCharacterMovement))))

(event EventOnRequestMoveTowards
  (params (position :type Vector%20%28by%20ref%29 :default "0, 0, 0"))
  (bind _output_get (Variables|Default|SetDestination (Math|Conversions|ToVector2D(Vector) position)))
  (AI|Navigation|MovetoLocation (AI|GetAIController self) (Math|Conversions|ToVector(Vector2D) _output_get (.Z (Class|KismetMathLibrary|BreakVector3f position))) 0.0 true false false true 0))

(fn ConstructionScript)